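; BP_Call_Elevator is an interactable elevator call actor tied to the BP_Ascenseur lift found in the level.
; Its construction script reads that lift's floor count and height to add a static mesh at each floor's vertical offset.
; On Interaction it prints the player's Z position and runs a timed move on the lift's SMLift01 component, with no target location wired.
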(event EventBeginPlay)

(event Collision|EventActorBeginOverlap
  (params (OtherActor :type Actor%20Object%20Reference)))

(event EventTick
  (params (DeltaSeconds :type Float%20%28single-precision%29)))

(event EventInteraction
  (Development|PrintString (Utilities|String|ToString(Float) (.z (Transformation|GetActorLocation (Game|GetPlayerCharacter 0)))))
  (bind _returnvalue (Actor|GetActorOfClass "/Game/Lift/Blueprints/BP_Ascenseur.BP_Ascenseur_C"))
  (Components|MoveComponentTo (Variables|/Game/Lift/Blueprints/BP_Ascenseur.BP_Ascenseur_C|GetSM_Lift01 _returnvalue) (Math|Vector|MakeVector 0.0 0.0 0.0) "0, 0, 0" false false 1.0 false))

(fn ConstructionScript
  (bind _returnvalue (Actor|GetActorOfClass "/Game/Lift/Blueprints/BP_Ascenseur.BP_Ascenseur_C"))
  (for _index (range 1 (Variables|/Game/Lift/Blueprints/BP_Ascenseur.BP_Ascenseur_C|GetNumberOfFloors _returnvalue))
    (AddComponent|AddStaticMeshComponent false (Math|Transform|MakeTransform (Math|Vector|MakeVector 0.0 0.0 (* (Variables|/Game/Lift/Blueprints/BP_Ascenseur.BP_Ascenseur_C|GetHauteur _returnvalue) _index 1e+02)) "0, 0, 0" "1.000000,1.000000,1.000000"))))