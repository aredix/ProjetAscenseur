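; BP_Ascenseur is an elevator Blueprint with an interaction-driven button menu.
; Its Construction Script adds one flattened static mesh per floor, stacked vertically at intervals set by Hauteur and counted by NumberOfFloors.
; The Interaction event creates the WBP_Bouton_Ascenseur widget, adds it to the viewport, switches the first player to UI-only input and shows the cursor.
; No cabin movement logic appears in this graph.
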(event EventInteraction
  (bind _returnvalue (Game|GetPlayerController 0))
  (bind _returnvalue_2 (UserInterface|CreateWidget "/Game/Lift/Blueprints/UI/WBP_Bouton_Ascenseur.WBP_Bouton_Ascenseur_C"))
  (UserInterface|Viewport|AddtoViewport _returnvalue_2 0)
  (Input|SetInputModeUIOnly _returnvalue 0 "DoNotLock" false)
  (Variables|/Script/Engine.PlayerController|SetbShowMouseCursor _returnvalue true))

(fn ConstructionScript
  (for _index (range 1 (Variables|Default|GetNumberOfFloors))
    (AddComponent|AddStaticMeshComponent false (Math|Transform|MakeTransform (Math|Vector|MakeVector -1.5e+02 -3e+01 (* (Variables|Default|GetHauteur) _index 1e+02)) "0, 0, 0" "3.000000,3.000000,0.100000"))))